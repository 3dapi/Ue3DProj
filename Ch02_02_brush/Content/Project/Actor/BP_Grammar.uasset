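; BP_Grammar is a scratch Blueprint that exercises basic scripting syntax: loops, arrays, functions, variables and flow-control nodes.
; BeginPlay overwrites ArrayValue with random floats and prints it, then appends ten more and prints again.
; Tick uses DoOnce to print a single range total from the local SumFunction loop.
; Most other nodes are disconnected samples of flow control, selection, casting and type conversion that never run.
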(event `self.ReceiveTick`
  (params (DeltaSeconds :type "Float (single-precision)"))
  (`/Engine/EditorBlueprintResources/StandardMacros.DoOnce` false
    (:`Completed`
      (bind _retsum (`self.SumFunction` 0 1000))
      (`KismetSystemLibrary.PrintString` (`KismetStringLibrary.Conv_IntToString` _retsum)))))

(event `self.ReceiveBeginPlay`
  (`|ExecutionSequence`
    (:`then_0`
      (for (_ _array_index) (`self.arrayValue`)
        (`KismetArrayLibrary.Array_Set` (`self.arrayValue`) _array_index (`KismetMathLibrary.RandomFloatInRange` 1.0 10000.0)))
      (for _array_element (`self.arrayValue`)
        (`KismetSystemLibrary.PrintString` (`KismetStringLibrary.Conv_DoubleToString` _array_element))))
    (:`then_1`
      (for _ (range 1 11)
        (`KismetArrayLibrary.Array_Add` (`self.arrayValue`) (`KismetMathLibrary.RandomFloatInRange` 1.0 10000.0)))
      (for _array_element_2 (`self.arrayValue`)
        (`KismetSystemLibrary.PrintString` (`KismetStringLibrary.Conv_DoubleToString` _array_element_2))))))

(fn `SumFunction`
  (params (argBegin :type Integer) (argEnd :type Integer))
  (returns (retSum :type Integer))
  (locals (localSum :type Integer))
  (for _index (range argBegin (+ argEnd 1))
    (set `local.localSum` (+ _index (`local.localSum`))))
  (return (`local.localSum`)))

(fn `UserConstructionScript`)